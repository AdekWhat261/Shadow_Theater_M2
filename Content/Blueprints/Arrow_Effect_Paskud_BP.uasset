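; Arrow effect actor that follows the mouse cursor and pushes balls it touches along the world X axis.
; Each tick it gets the EffectControl_Controller_BP player controller and moves to the cursor's hit location on the Camera trace channel.
; On overlap with a Ball_BP, it applies an impulse to the ball's Sharik2 component, using only the X part of the Cylinder's forward vector scaled by ImpulseStrength.
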(event Collision|EventActorBeginOverlap
  (params (OtherActor :type Actor%20Object%20Reference))
  (bind _asball_bp (Utilities|Casting|CastToBall_BP OtherActor))
  (Physics|AddImpulse (Variables|/Game/Blueprints/Ball_BP.Ball_BP_C|GetSharik%202 _asball_bp) (Math|Vector|MakeVector (.x (* (Math|Vector|MakeVector (.x (Math|Vector|GetForwardVector (Transformation|GetWorldRotation (Variables|Default|GetCylinder)))) 0.0 0.0) (Variables|Default|GetImpulse%20Strength))) 0.0 0.0) "None" false))

(event EventTick
  (params (DeltaSeconds :type Float%20%28single-precision%29))
  (bind _returnvalue (Class|InputDeviceLibrary|GetPlayerControllerfromInputDevice))
  (bind _aseffect_control_controller_bp (Utilities|Casting|CastToEffectControl_Controller_BP _returnvalue))
  (Transformation|SetActorLocation (.Location (Collision|BreakHitResult (.HitResult (Game|Player|GetHitResultUnderCursorbyChannel _aseffect_control_controller_bp "TraceTypeQuery2" true)))) false false))

(fn ConstructionScript)