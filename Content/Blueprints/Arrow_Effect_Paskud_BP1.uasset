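; Placeable arrow effect actor that pushes the ball when it enters the actor's box.
; Once IsPlaced is set, a Ball_BP overlap applies an impulse along world X only, scaled by the actor's forward X and ImpulsePower.
; The E key sets rotation from the current roll with a zero offset.
; Left mouse press and release each spawn an Arrow_Effect_Paskud_BP at the world origin.
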(event OnComponentBeginOverlap(Box)
  (params (OverlappedComponent :type Primitive%20Component%20Object%20Reference) (OtherActor :type Actor%20Object%20Reference) (OtherComp :type Primitive%20Component%20Object%20Reference) (OtherBodyIndex :type Integer) (bFromSweep :type Boolean) (SweepResult :type Hit%20Result%20Structure%20%28by%20ref%29))
  (if (Variables|Default|GetIsPlaced)
    ;[1 0.9939 0.3027] Импульс шарику
    (bind _asball_bp (Utilities|Casting|CastToBall_BP OtherActor))
    (Physics|AddImpulse (Variables|/Game/Blueprints/Ball_BP.Ball_BP_C|GetBall _asball_bp) (Math|Vector|MakeVector (.x (* (Math|Vector|MakeVector (.x (Math|Vector|GetForwardVector (Transformation|GetActorRotation))) 0.0 0.0) (Variables|Default|GetImpulse%20Power))) 0.0 0.0) "None" false)))

(event Input|KeyboardEvents|E
  (params (Key :type Key%20Structure :default "None"))
  (:Pressed
    (Transformation|SetActorRotation (Math|Rotator|MakeRotator (+ (.roll (Transformation|GetActorRotation)) 0.0) 0.0 0.0))))

(event Input|KeyboardEvents|Q
  (params (Key :type Key%20Structure :default "None")))

(event Input|MouseEvents|LeftMouseButton
  (params (Key :type Key%20Structure :default "None"))
  (:Pressed
    (Game|SpawnActorfromClass "/Game/Blueprints/Arrow_Effect_Paskud_BP.Arrow_Effect_Paskud_BP_C" (Math|Conversions|ToTransform(Vector) "0, 0, 0") "Undefined" "MultiplyWithRoot" 0 0 :!label _label))
  (:Released
    (goto _label)))

(fn ConstructionScript)