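; Input controller Blueprint that spawns arrow effects and switches on physics for a referenced Ball_BP.
; BeginPlay casts and stores the Ball reference and sets the IsPsyhics flag.
; Left mouse spawns Arrow_Effect_BP using the ball's rotation and only the X component of its location.
; Space press enables physics simulation on the ball through an always-true branch, while release only clears the flag, leaving simulation on.
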(event EventBeginPlay
  (bind _asball_bp (Utilities|Casting|CastToBall_BP (Variables|Default|GetBall)))
  (Variables|Default|SetBall _asball_bp)
  (Variables|Default|SetIsPsyhics true))

(event Input|MouseEvents|LeftMouseButton
  (params (Key :type Key%20Structure))
  (:Pressed
    (Game|SpawnActorfromClass "/Game/Blueprints/Arrow_Effect_BP.Arrow_Effect_BP_C" (Math|Transform|MakeTransform (Math|Vector|MakeVector (.x (Transformation|GetWorldLocation (Variables|/Script/Engine.Actor|GetRootComponent (Variables|Default|GetBall)))) 0.0 0.0) (Transformation|GetWorldRotation (Variables|/Script/Engine.Actor|GetRootComponent (Variables|Default|GetBall))) "1.000000,1.000000,1.000000") "Undefined" "MultiplyWithRoot" 0 0)))

(event Input|KeyboardEvents|SpaceBar
  (params (Key :type Key%20Structure))
  (:Pressed
    (Utilities|Casting|CastToBall_BP (Variables|Default|GetBall))
    (if true
      (Variables|Default|SetIsPsyhics true)
      (Physics|SetSimulatePhysics (Variables|/Game/Blueprints/Ball_BP.Ball_BP_C|GetBall (Variables|Default|GetBall)) true)
      (else
        (Variables|Default|SetIsPsyhics false))))
  (:Released
    (Variables|Default|SetIsPsyhics false)))

(fn ConstructionScript)